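; BP_Test is a lab test actor with a trigger-driven moving ceiling lamp and a key-controlled light.
; Overlapping the trigger box plays a timeline that drives the lamp mesh's relative Z height at a fixed doubled scale.
; Pressing Z applies the Intensity variable to the light, then after a short delay zeroes both.
; Intensity is never restored, so later presses leave the light dark.
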(event `self.trigger_box.OnComponentBeginOverlap`
  (params (OverlappedComponent :type "PrimitiveComponent Object Reference") (OtherActor :type "Actor Object Reference") (OtherComp :type "PrimitiveComponent Object Reference") (OtherBodyIndex :type Integer) (bFromSweep :type Boolean) (SweepResult :type "HitResult Structure (by ref)"))
  (bind (_direction _z_value) (`Timeline|Timeline` :`NewTime` 0.0)
    (:`Update`
      (`SceneComponent.K2_SetRelativeTransform` (`self.SM_Lamp_Ceiling`) (`KismetMathLibrary.MakeTransform` (`KismetMathLibrary.MakeVector` 0.0 0.0 _z_value) (struct) (2.0 2.0 2.0)) false false))))

(event `Key|Z`
  (params (Key :type "Key Structure"))
  (:`Pressed`
    (`LightComponent.SetIntensity` (`self.light`) (`self.intensity`))
    (`KismetSystemLibrary.Delay` 1.0)
    (set `self.intensity` 0.0)
    (`LightComponent.SetIntensity` (`self.light`) (`self.intensity`))))

(fn `UserConstructionScript`)